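; Procedural building actor that assembles a multi-floor structure from modular wall and ground meshes in its construction script.
; Each FloorInformation entry sets a floor's length, width, offset and per-segment meshes for four walls, with arrays resized automatically and FillWall replacing empty slots.
; Static mesh components are spaced by their bounds, with a temporary ground tile measuring the floor grid step.
; BuildingChangeAllWalls overwrites every wall slot with AllWalls.
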(event Custom|Building%20Change%20All%20Walls
  (bind _floorinformation (Variables|Building|GetFloorInformation))
  (bind _allwalls (Variables|Default|GetAllWalls))
  (for (_array_element _array_index) _floorinformation
    (Utilities|Array|SetArrayElem _floorinformation _array_index (Utilities|Struct|MakeS_BasicBuildingFloorData (.Length (Utilities|Struct|BreakS_BasicBuildingFloorData _array_element)) (.Width (Utilities|Struct|BreakS_BasicBuildingFloorData _array_element)) (.Offset (Utilities|Struct|BreakS_BasicBuildingFloorData _array_element)) (CallFunction|ChangeAll (.Wall1Meshes (Utilities|Struct|BreakS_BasicBuildingFloorData _array_element)) _allwalls) (CallFunction|ChangeAll (.Wall2Meshes (Utilities|Struct|BreakS_BasicBuildingFloorData _array_element)) _allwalls) (CallFunction|ChangeAll (.Wall3Meshes (Utilities|Struct|BreakS_BasicBuildingFloorData _array_element)) _allwalls) (CallFunction|ChangeAll (.Wall4Meshes (Utilities|Struct|BreakS_BasicBuildingFloorData _array_element)) _allwalls)))))

(fn ConstructionScript
  (CallFunction|ResizeArray)
  (for (_array_element _array_index) (Variables|Building|GetFloorInformation)
    (CallFunction|SingleWall (.length _array_element) (.width _array_element) (.offset _array_element) (.wall1meshes _array_element) (.wall2meshes _array_element) (.wall3meshes _array_element) (.wall4meshes _array_element))
    (CallFunction|SingleFloor (.length _array_element) (.width _array_element) _array_index)))

(fn SingleWall
  (params (Length :type Integer) (Width :type Integer) (Offset :type Vector) (Wall1 :type Array%20of%20Static%20Mesh%20Object%20References) (Wall2 :type Array%20of%20Static%20Mesh%20Object%20References) (Wall3 :type Array%20of%20Static%20Mesh%20Object%20References) (Wall4 :type Array%20of%20Static%20Mesh%20Object%20References))
  (for _index (range 1 Length)
    (bind (_returnvalue _extendx) (CallFunction|AddStaticMesh (.Output (CallFunction|SelectWallMesh Wall1 _index)) "1.000000,1.000000,1.000000"))
    (CallFunction|ModifyStaticMesh _returnvalue (+ (* (.ReturnValue (CallFunction|SelectWallMesh Wall1 _index)) _extendx) (.x Offset)) (.y Offset) (.z Offset) "1.000000,1.000000,1.000000" (Variables|Floor|Walls|Rotation|GetWall1Rotation))
    (Variables|Private|SetXDistance (* _index _extendx)))
  (for _index_2 (range 1 Width)
    (bind (_returnvalue_2 _extendx_2) (CallFunction|AddStaticMesh (.Output (CallFunction|SelectWallMesh Wall3 _index_2)) "1.000000,1.000000,1.000000"))
    (CallFunction|ModifyStaticMesh _returnvalue_2 (.x Offset) (+ (* _index_2 _extendx_2) (.y Offset)) (.z Offset) "1.000000,1.000000,1.000000" (Variables|Floor|Walls|Rotation|GetWall2Rotation))
    (Class|UEExtendedConditionLibrary|IsBiggerThanZero (+ (* _index_2 _extendx_2) (.y Offset))
      (:OutTrue
        (Variables|Private|SetYDistance (+ (* _index_2 _extendx_2) (.y Offset))))))
  (for _index_3 (range 1 Width)
    (bind (_returnvalue_3 _extendx_3) (CallFunction|AddStaticMesh (.Output (CallFunction|SelectWallMesh Wall4 _index_3)) "1.000000,1.000000,1.000000"))
    (CallFunction|ModifyStaticMesh _returnvalue_3 (+ (Variables|Private|GetXDistance) (.x Offset)) (+ (* (.ReturnValue (CallFunction|SelectWallMesh Wall4 _index_3)) _extendx_3) (.y Offset)) (.z Offset) "1.000000,1.000000,1.000000" (Variables|Floor|Walls|Rotation|GetWall3Rotation)))
  (for _index_4 (range 1 Length)
    (bind (_returnvalue_4 _extendx_4) (CallFunction|AddStaticMesh (.Output (CallFunction|SelectWallMesh Wall2 _index_4)) "1.000000,1.000000,1.000000"))
    (CallFunction|ModifyStaticMesh _returnvalue_4 (+ (* _index_4 _extendx_4) (.x Offset)) (+ (.y Offset) (Variables|Private|GetYDistance)) (.z Offset) "1.000000,1.000000,1.000000" (Variables|Floor|Walls|Rotation|GetWall4Rotation))))

(fn AddStaticMesh
  (params (NewMesh :type Static%20Mesh%20Object%20Reference) (Relative%20Transform%20Scale :type Vector :default "1.000000,1.000000,1.000000"))
  (bind _returnvalue (AddComponent|AddStaticMeshComponent false (Math|Transform|MakeTransform "0, 0, 0" "0, 0, 0" Relative%20Transform%20Scale)))
  (Components|StaticMesh|SetStaticMesh _returnvalue NewMesh)
  (return _returnvalue (Class|UEExtendedMathLibrary|FloatMultiplybyTwo (.x (.BoxExtent (Collision|GetComponentBounds _returnvalue))))))

(fn ModifyStaticMesh
  (params (MeshComp :type Static%20Mesh%20Component%20Object%20Reference) (New%20Location%20X :type Float%20%28single-precision%29) (New%20Location%20Y :type Float%20%28single-precision%29) (New%20Location%20Z :type Float%20%28single-precision%29) (NewScale3D :type Vector :default "1.000000,1.000000,1.000000") (New%20Rotation%20Z :type Float%20%28single-precision%29))
  (Transformation|SetRelativeLocation MeshComp (Math|Vector|MakeVector New%20Location%20X New%20Location%20Y New%20Location%20Z) false false)
  (CallFunction|SetCompRelativeRotationZ MeshComp New%20Rotation%20Z))

(fn SingleFloor
  (params (Length :type Integer) (Width :type Integer) (Index :type Integer))
  (bind _goundoffset (Variables|Floor|Ground|GetGoundOffset))
  (bind _output (Utilities|Array|Get(acopy) _goundoffset Index))
  (bind (_returnvalue _extendx) (CallFunction|AddStaticMesh (Variables|Floor|Ground|GetGroundMesh) (Variables|Floor|Ground|GetGroundScale)))
  (LocalVariables|SetNewLocalVar_0 _returnvalue)
  (Variables|Private|SetGroundDistance _extendx)
  (for _index (range 1 (Class|UEExtendedMathLibrary|IntMinusOne Length))
    (for _index_2 (range 1 (Class|UEExtendedMathLibrary|IntMinusOne Width))
      (bind _returnvalue_2 (CallFunction|AddStaticMesh (Variables|Floor|Ground|GetGroundMesh) (Variables|Floor|Ground|GetGroundScale)))
      (CallFunction|ModifyStaticMesh _returnvalue_2 (+ (* _index (Variables|Private|GetGroundDistance)) (.x _output)) (+ (* _index_2 (Variables|Private|GetGroundDistance)) (.y _output)) (.z _output) "1.000000,1.000000,1.000000" 0.0)))
  (Components|DestroyComponent (LocalVariables|GetNewLocalVar_0)))

(fn GetWallPositionwithOffset
  (params (InputX :type Integer) (InputY :type Integer) (Offset :type Vector) (Distance :type Float%20%28single-precision%29))
  (return 0.0 0.0 0.0))

(fn ResizeArray
  (bind _floorinformation (Variables|Building|GetFloorInformation))
  (for (_array_element _array_index) _floorinformation
    (LocalVariables|SetLength (.length _array_element))
    (LocalVariables|SetWidth (.width _array_element))
    (LocalVariables|SetOffset (.offset _array_element))
    (bind _output_get (LocalVariables|SetWall1 (.wall1meshes _array_element)))
    (Utilities|Array|Resize _output_get (LocalVariables|GetLength))
    (bind _output_get_2 (LocalVariables|SetWall4 (.wall4meshes _array_element)))
    (Utilities|Array|Resize _output_get_2 (LocalVariables|GetLength))
    (bind _output_get_3 (LocalVariables|SetWall2 (.wall2meshes _array_element)))
    (Utilities|Array|Resize _output_get_3 (LocalVariables|GetWidth))
    (bind _output_get_4 (LocalVariables|SetWall3 (.wall3meshes _array_element)))
    (Utilities|Array|Resize _output_get_4 (LocalVariables|GetWidth))
    (Utilities|Array|SetArrayElem _floorinformation _array_index (Utilities|Struct|MakeS_BasicBuildingFloorData (LocalVariables|GetLength) (LocalVariables|GetWidth) (LocalVariables|GetOffset) (LocalVariables|GetWall1) (LocalVariables|GetWall2) (LocalVariables|GetWall3) (LocalVariables|GetWall4))))
  (Utilities|Array|Resize (Variables|Floor|Ground|GetGoundOffset) (Utilities|Array|Length (Variables|Building|GetFloorInformation))))

(fn ChangeAll
  (params (MeshArray :type Array%20of%20Static%20Mesh%20Object%20References) (NewItem :type Static%20Mesh%20Object%20Reference%20%28by%20ref%29))
  (for _array_element MeshArray
    (Utilities|Array|Add (LocalVariables|GetNewLocalVar_2) NewItem))
  (return (LocalVariables|GetNewLocalVar_2)))

(fn AddWall
  (params (Value :type Integer) (Array :type Array%20of%20Static%20Mesh%20Object%20References) (Offset :type Vector)))

(fn SelectWallMesh
  (params (Array :type Array%20of%20Static%20Mesh%20Object%20References) (index :type Integer))
  (bind _output (Utilities|Array|Get(acopy) Array index))
  (return (select (Utilities|IsValid _output) _output (Variables|Floor|Walls|GetFillWall)) (Class|UEExtendedMathLibrary|IntMinusOne index)))