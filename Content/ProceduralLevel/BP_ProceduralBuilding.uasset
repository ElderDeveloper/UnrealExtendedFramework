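; Procedural building actor that assembles a rectangular, multi-floor building from static mesh components in its construction script.
; For each floor, SingleFloorWalls lines four sides with wall meshes, then SingleFloor fills a grid of ground meshes.
; Wall spacing comes from the mesh's bounds width plus an adjustable offset, and the ground grid reuses the measured X-wall width.
; SingleCeiling is defined but never called, and the event graph is empty.
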(event EventBeginPlay)

(event Collision|EventActorBeginOverlap
  (params (OtherActor :type Actor%20Object%20Reference)))

(event EventTick
  (params (DeltaSeconds :type Float%20%28single-precision%29)))

(fn ConstructionScript
  (for _index (range 1 (Variables|Floor|GetFloorAmount))
    (CallFunction|SingleFloorWalls _index)
    (CallFunction|SingleFloor _index)))

(fn SingleFloorWalls
  (params (WallFloor :type Integer))
  (LocalVariables|SetFloor (Class|UEExtendedMathLibrary|IntMinusOne WallFloor))
  (for _index (range 1 (Variables|Walls|GetWallX))
    (bind (_returnvalue _extendx) (CallFunction|AddStaticMesh (Variables|Walls|GetWallMesh)))
    (CallFunction|ModifyStaticMesh _returnvalue (* (Class|UEExtendedMathLibrary|IntMinusOne _index) (+ _extendx (Variables|Default|GetPlusXExtend))) 0.0 (Variables|Walls|GetWallScale) (LocalVariables|GetFloor) (Variables|Walls|GetXWallsRotation))
    (Variables|Default|SetWallXDistance _extendx))
  (for _index_2 (range 1 (Variables|Walls|GetWallY))
    (bind (_returnvalue_2 _extendx_2) (CallFunction|AddStaticMesh (Variables|Walls|GetWallMesh)))
    (CallFunction|ModifyStaticMesh _returnvalue_2 0.0 (* _index_2 (+ _extendx_2 (Variables|Default|GetPlusXExtend))) (Variables|Walls|GetWallScale) (LocalVariables|GetFloor) (Variables|Walls|GetYWallsRotation))
    (Variables|Default|SetWallYDistance (* _index_2 (+ _extendx_2 (Variables|Default|GetPlusXExtend)))))
  (for _index_3 (range 1 (Variables|Walls|GetWallY))
    (bind (_returnvalue_3 _extendx_3) (CallFunction|AddStaticMesh (Variables|Walls|GetWallMesh)))
    (CallFunction|ModifyStaticMesh _returnvalue_3 (* (Class|UEExtendedMathLibrary|IntMinusOne (Variables|Walls|GetWallX)) (Variables|Default|GetWallXDistance)) (* _index_3 (+ _extendx_3 (Variables|Default|GetPlusXExtend))) (Variables|Walls|GetWallScale) (LocalVariables|GetFloor) (Variables|Walls|GetYWallsRotation)))
  (for _index_4 (range 1 (Variables|Walls|GetWallX))
    (bind (_returnvalue_4 _extendx_4) (CallFunction|AddStaticMesh (Variables|Walls|GetWallMesh)))
    (CallFunction|ModifyStaticMesh _returnvalue_4 (* (Class|UEExtendedMathLibrary|IntMinusOne _index_4) (+ _extendx_4 (Variables|Default|GetPlusXExtend))) (* (Variables|Walls|GetWallY) (Variables|Default|GetWallXDistance)) (Variables|Walls|GetWallScale) (LocalVariables|GetFloor) (Variables|Walls|GetXWallsRotation))))

(fn SingleFloor
  (params (GroundFloor :type Integer))
  (LocalVariables|SetFloor (Class|UEExtendedMathLibrary|IntMinusOne GroundFloor))
  (for _index (range 0 (Variables|Walls|GetWallX))
    (for _index_2 (range 0 (Variables|Walls|GetWallY))
      (bind _returnvalue (AddComponent|AddStaticMeshComponent false (Math|Transform|MakeTransform (Math|Vector|MakeVector (* _index (Variables|Default|GetWallXDistance)) (* _index_2 (Variables|Default|GetWallXDistance)) (* (LocalVariables|GetFloor) (Variables|Floor|GetFloorHeight))) "0, 0, 0" (Variables|Ground|GetGroundScale))))
      (Components|StaticMesh|SetStaticMesh _returnvalue (Variables|Ground|GetGroundMesh)))))

(fn SingleCeiling
  (params (GroundFloor :type Integer))
  (LocalVariables|SetFloor (Class|UEExtendedMathLibrary|IntMinusOne GroundFloor))
  (for _index (range 0 (Variables|Walls|GetWallX))
    (for _index_2 (range 0 (Variables|Walls|GetWallY))
      (bind _returnvalue (AddComponent|AddStaticMeshComponent false (Math|Transform|MakeTransform (Math|Vector|MakeVector (* _index (Variables|Walls|GetWallDistance)) (* _index_2 (Variables|Walls|GetWallDistance)) (* (LocalVariables|GetFloor) (Variables|Floor|GetFloorHeight))) "0, 0, 0" (Variables|Ground|GetGroundScale))))
      (Components|StaticMesh|SetStaticMesh _returnvalue (Variables|Ground|GetGroundMesh)))))

(fn ModifyStaticMesh
  (params (MeshComp :type Static%20Mesh%20Component%20Object%20Reference) (New%20Location%20X :type Float%20%28single-precision%29) (New%20Location%20Y :type Float%20%28single-precision%29) (Relative%20Transform%20Scale :type Vector) (Floor :type Integer) (New%20Rotation%20Z :type Float%20%28single-precision%29))
  (Transformation|SetRelativeScale3D MeshComp Relative%20Transform%20Scale)
  (Transformation|SetRelativeLocation MeshComp (Math|Vector|MakeVector New%20Location%20X New%20Location%20Y (+ (* Floor (Variables|Floor|GetFloorHeight)) (Variables|Walls|GetWallStartHeight))) false false)
  (CallFunction|SetCompRelativeRotationZ MeshComp New%20Rotation%20Z))

(fn GetBoxExtendX
  (params (Component :type Scene%20Component%20Object%20Reference))
  (return (Class|UEExtendedMathLibrary|FloatMultiplybyTwo (.x (.BoxExtent (Collision|GetComponentBounds Component))))))

(fn AddStaticMesh
  (params (NewMesh :type Static%20Mesh%20Object%20Reference))
  (bind _returnvalue (AddComponent|AddStaticMeshComponent false))
  (Components|StaticMesh|SetStaticMesh _returnvalue NewMesh)
  (return _returnvalue (CallFunction|GetBoxExtendX _returnvalue)))